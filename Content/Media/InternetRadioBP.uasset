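; Internet radio Blueprint that streams a list of stations through a Media Player and Media Sound Component.
; BeginPlay shows the main widget and sets the base sound mix; R opens the radio widget with UI-only input and starts the current station, and Q quits.
; Exposes play, pause and wrap-around next/previous station functions, with volume applied through a Sound Mix class override on the radio's Sound Class.
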(event `self.ReceiveBeginPlay`
  (bind _returnvalue (`|CreateWidget` "/Game/Media/MainWidget.MainWidget_C"))
  (bind _output_get (set `self.MainWidget` _returnvalue))
  (`UserWidget.AddToViewport` _output_get 0)
  (`AddComponent|NODE_AddMediaSoundComponent-0`)
  (`GameplayStatics.SetBaseSoundMix` "/Game/Media/InternetRadioSM.InternetRadioSM")
  (`self.EnableInput` (`GameplayStatics.GetPlayerController` 0)))

(event `Key|Q`
  (params (Key :type "Key Structure"))
  (:`Pressed`
    (`KismetSystemLibrary.QuitGame` null "Quit")))

(event `Key|R`
  (params (Key :type "Key Structure"))
  (:`Pressed`
    (`self.TurnOnRadio`)))

(fn `ChangeVolumeRadio`
  (params (VolumeLevel :type "Float (double-precision)"))
  (set `self.VolumeLevel` VolumeLevel)
  (`GameplayStatics.SetSoundMixClassOverride` "/Game/Media/InternetRadioSM.InternetRadioSM" "/Game/Media/InternetradioSC.InternetRadioSC" (`self.VolumeLevel`)))

(fn `NewStation`
  (`MediaPlayer.OpenSource` (`self.MediaPlayer`) (`|GetArrayItem` (`self.StationsList`) (`self.StationIndex`))))

(fn `NextStation`
  (set `self.StationIndex` (mod (+ (`self.StationIndex`) 1) (`KismetArrayLibrary.Array_Length` (`self.StationsList`))))
  (`self.NewStation`))

(fn `PauseRadio`
  (`MediaPlayer.Pause` (`self.MediaPlayer`)))

(fn `PlayRadio`
  (`MediaPlayer.Play` (`self.MediaPlayer`)))

(fn `PreviousStation`
  (bind _returnvalue (- (`self.StationIndex`) 1))
  (set `self.StationIndex` (select `bool` (< _returnvalue 0) :`false` _returnvalue :`true` (`KismetArrayLibrary.Array_LastIndex` (`self.StationsList`))))
  (`self.NewStation`))

(fn `TurnOnRadio`
  (`self.InternetRadioWidget`
    (:`then`
      _)
    (:`else`
      (bind _returnvalue (`|CreateWidget` "/Game/Media/InternetRadioWidget.InternetRadioWidget_C"))
      (set `self.InternetRadioWidget` _returnvalue)))
  (`UserWidget.AddToViewport` (`self.InternetRadioWidget`) 0)
  (`self.NewStation`)
  (`self.ChangeVolumeRadio` (`self.VolumeLevel`))
  (set `PlayerController.bShowMouseCursor` true (`GameplayStatics.GetPlayerController` 0))
  (`WidgetBlueprintLibrary.SetInputMode_UIOnlyEx` (`GameplayStatics.GetPlayerController` 0)))

(fn `UserConstructionScript`)